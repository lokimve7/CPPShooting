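; BP_Only_Player is a player-controlled shooter actor that moves on its right/up plane and fires bullets.
; Tick combines the Horizontal and Vertical inputs into a normalized direction, then applies position plus velocity times delta time at a fixed speed.
; Movement sets the location directly without sweeping, so it does not stop at obstacles.
; Releasing the Fire action spawns a BP_Only_Bullet at the FirePos component's world transform.
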(event `self.ReceiveTick`
  (params (DeltaSeconds :type "Float (single-precision)"))
  (`self.K2_SetActorLocation` (+ (* DeltaSeconds (* (`KismetMathLibrary.Normal` (+ (* (`self.GetActorRightVector`) (`self.GetInputAxisValue`)) (* (`self.GetActorUpVector`) (`self.GetInputAxisValue`)))) 500.0)) (`self.K2_GetActorLocation`))))

(event `InputAction|Fire`
  (params (Key :type "Key Structure"))
  ;[1 1 1] 총알 발사
  (:`Released`
    (`|SpawnActorFromClass` "/Game/Blueprints/BP_Only_Bullet.BP_Only_Bullet_C" (`SceneComponent.K2_GetComponentToWorld` (`self.FirePos`)) "Undefined" "OverrideRootScale" null null)))

(fn `UserConstructionScript`)