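; BP_Only_Enemy is a simple enemy that homes in on the player.
; On BeginPlay, it finds the BP_Only_Player actor as its Target if that is not already valid.
; Each Tick, it recomputes the normalized direction to Target and moves by Speed scaled by delta time, with no sweep and no validity check on Target.
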(event `self.ReceiveBeginPlay`
  (`/Engine/EditorBlueprintResources/StandardMacros.IsValid` (`self.target`)
    (:`Is Not Valid`
      ;[1 1 1] 플레이어 찾자.
      (bind _returnvalue (`GameplayStatics.GetActorOfClass` "/Game/Blueprints/BP_Only_Player.BP_Only_Player_C"))
      (set `self.target` _returnvalue))))

(event `self.ReceiveTick`
  (params (DeltaSeconds :type "Float (single-precision)"))
  ;[1 1 1] Target을 향하는 방향을 구하자
  (set `self.dir` (`KismetMathLibrary.Normal` (- (`self.K2_GetActorLocation` (`self.target`)) (`self.K2_GetActorLocation`))))
  (`self.K2_SetActorLocation` (+ (`self.K2_GetActorLocation`) (* DeltaSeconds (* (`self.dir`) (`self.speed`))))))

(fn `UserConstructionScript`)